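; Knight1 is an AI-moved knight that approaches the player and triggers a screen fade when it arrives.
; BeginPlay caches the player and Knight2, adding a FadeInOut widget per Knight2 found.
; Tick yaws the knight along the player-to-knight direction and rebinds Move to Knight2's MoveToCharacter event every frame.
; Move runs AIMoveTo toward the player, playing the fade on success and retrying itself on failure.
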(event Custom|Move
  (AI|AIMoveTo self "0, 0, 0" (Game|Player|GetPlayerPawn 0) 5.0 false
    (:OnSuccess
      (Default|PlayFadeAnimation (Variables|Default|GetFadeInOut)))
    (:OnFail
      (CallFunction|Move))))

(event EventBeginPlay
  (bind _astest_character (Utilities|Casting|CastToTestCharacter (Game|GetPlayerCharacter 0)))
  (Variables|Default|SetPlayer _astest_character)
  (bind _outactors (Actor|GetAllActorsOfClass "/Game/PapertownProject/Blueprints/Character/Knight2.Knight2_C"))
  (for _array_element _outactors
    (Variables|Default|SetKnight2 _array_element)
    (bind _returnvalue (UserInterface|CreateWidget "/Game/PapertownProject/Blueprints/UI/FadeInOut.FadeInOut_C"))
    (bind _output_get (Variables|Default|SetFadeInOut _returnvalue))
    (UserInterface|Viewport|AddtoViewport _output_get 0)))

(event EventTick
  (params (DeltaSeconds :type Float%20%28single-precision%29))
  (Transformation|SetActorRotation (Math|Rotator|MakeRotator 0.0 0.0 (.yaw (Math|Rotator|FindLookatRotation (Transformation|GetActorLocation (Game|GetPlayerCharacter 0)) (Transformation|GetActorLocation)))))
  (EventDispatchers|BindEventtoMovetoCharacter (Variables|Default|GetKnight2) (delegate Custom|Move)))

(fn ConstructionScript)
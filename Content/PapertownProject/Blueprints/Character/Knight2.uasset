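; Knight2 is an AI-moved pawn that chases the player once triggered by a MoveToCharacter event.
; BeginPlay caches the player as TestCharacter and stores the last Knight1 found in the level.
; Tick sets yaw along the player-to-knight direction, facing away from the player, and rebinds Move to MoveToCharacter every frame.
; Move runs AI MoveTo toward the player pawn and calls itself again on failure.
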(event Custom|Move
  (AI|AIMoveTo self "0, 0, 0" (Game|Player|GetPlayerPawn 0) 5.0 false
    (:OnFail
      (CallFunction|Move))))

(event EventBeginPlay
  (bind _astest_character (Utilities|Casting|CastToTestCharacter (Game|GetPlayerCharacter 0)))
  (Variables|Default|SetPlayer _astest_character)
  (bind _outactors (Actor|GetAllActorsOfClass "/Game/PapertownProject/Blueprints/Character/Knight1.Knight1_C"))
  (for _array_element _outactors
    (Variables|Default|SetKnight1 _array_element)))

(event EventTick
  (params (DeltaSeconds :type Float%20%28single-precision%29))
  (Transformation|SetActorRotation (Math|Rotator|MakeRotator 0.0 0.0 (.yaw (Math|Rotator|FindLookatRotation (Transformation|GetActorLocation (Game|GetPlayerCharacter 0)) (Transformation|GetActorLocation)))))
  (EventDispatchers|BindEventtoMovetoCharacter (delegate Custom|Move)))

(fn ConstructionScript)